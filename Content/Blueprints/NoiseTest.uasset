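; Test actor that generates a grayscale noise texture on BeginPlay.
; A fractal gradient noise generator is sampled over a Size-based 2D grid, and the absolute value of each sample becomes a grey color in an array.
; Maketexture turns that array into a texture stored in Tex.
; Each sample is also printed on screen, with the noise value itself wired in as the display duration.
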(event `self.ReceiveBeginPlay`
  (bind _size (`self.Size`))
  (bind _col (`self.Col`))
  (bind _output_get (set `self.Noise` (`UFNBlueprintFunctionLibrary.CreateFractalNoiseGenerator` self "FractalGradient")))
  ;[1 1 1] y
  (for _index (range (+ _size 1))
    ;[1 1 1] x
    (for _index_2 (range (+ _size 1))
      (bind _returnvalue (`UFNNoiseGenerator.GetNoise2D` _output_get (`KismetMathLibrary.Conv_IntToDouble` _index_2) (`KismetMathLibrary.Conv_IntToDouble` _index)))
      (`KismetSystemLibrary.PrintString` (`KismetStringLibrary.Conv_DoubleToString` _returnvalue) true true (struct :`G` 0.66 :`B` 1.0 :`A` 1.0) _returnvalue)
      (bind _returnvalue_2 (`KismetMathLibrary.Abs` _returnvalue))
      (`KismetArrayLibrary.Array_Add` _col (`KismetMathLibrary.Conv_LinearColorToColor` (`KismetMathLibrary.MakeColor` _returnvalue_2 _returnvalue_2 _returnvalue_2)))))
  (bind _returnvalue_3 (`TestProceduralMesh.Maketexture` _col (`self.Size`) self))
  (set `self.Tex` _returnvalue_3))

(fn `UserConstructionScript`)